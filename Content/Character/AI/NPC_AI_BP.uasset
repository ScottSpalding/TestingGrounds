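; AI controller for guard NPCs that starts the guard behavior tree on the patrol blackboard at BeginPlay.
; AI perception updates feed the blackboard enemy key, storing the actor when it is sensed and clearing the key when sensing fails.
; Only actors without the "Enemy" tag affect the key, so tagged actors are ignored.
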(event `self.ReceiveBeginPlay`
  (bind _blackboardcomponent (`self.UseBlackboard` "/Game/Character/AI/PatrolData.PatrolData"))
  (`self.RunBehaviorTree` "/Game/Character/AI/GuardBehaviorTree.GuardBehaviorTree")
  (set `self.BlackboardComp` _blackboardcomponent))

(event `self.AIPerception.OnTargetPerceptionUpdated`
  (params (Actor :type "Actor Object Reference") (Stimulus :type "AIStimulus Structure"))
  (`self.Update Blackboard Enemy Key` Actor Stimulus))

(fn `Update Blackboard Enemy Key`
  (params (NewlySensed :type "Object Object Reference") (AIStimulus :type "AIStimulus Structure (by ref)"))
  (bind _enemykey (`self.EnemyKey`))
  (bind _blackboardcomp (`self.BlackboardComp`))
  (bind _asactor (cast `Actor` NewlySensed))
  (if (`self.ActorHasTag` _asactor "Enemy")
    _
    (elif (`.bSuccessfullySensed` (break `AIStimulus` AIStimulus))
      (`BlackboardComponent.SetValueAsObject` _blackboardcomp _enemykey NewlySensed)
      (else
        (`BlackboardComponent.ClearValue` _blackboardcomp _enemykey)))))

(fn `UserConstructionScript`)