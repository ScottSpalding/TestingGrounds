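; Game mode for an infinite terrain game that spawns a chain of BP_Tile actors and keeps the score.
; On BeginPlay it populates a nav mesh bounds volume pool, then spawns the initial tiles.
; Each spawned tile receives the pool and supplies its attach location as the next tile's spawn transform.
; NewTileConquered increments the score, which GetScore exposes.
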(event `self.ReceiveBeginPlay`
  (`self.PopulateBoundsVolumePool`)
  (for _ (range 4)
    (`self.Spawn Tile`)
    (`KismetSystemLibrary.PrintString` "Spawning Tile")))

(fn `GetScore`
  (returns (Score :type Integer))
  (return (`self.Score`)))

(fn `NewTileConquered`
  (`/Engine/EditorBlueprintResources/StandardMacros.IncrementInt` (`self.Score`)))

(fn `Spawn Tile`
  (bind _returnvalue (`|SpawnActorFromClass` "/Game/Terrain/BP_Tile.BP_Tile_C" (`self.NewTileTransform`) "Undefined" "OverrideRootScale" null null))
  (`Tile.SetPool` _returnvalue (`self.NavMeshBoundsVolumePool`))
  (bind _attach_transform (`/Game/Terrain/BP_Tile.Get Attach Location` _returnvalue))
  (set `self.NewTileTransform` _attach_transform))

(fn `UserConstructionScript`)